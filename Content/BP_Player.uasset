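; Player character with movement, shooting, slow motion and game timers.
; BeginPlay attaches a weapon and adds HUD widgets; left click shakes the camera and calls a spawn at the muzzle with no class shown.
; Right click toggles global time dilation while held, with stamina drained and recharged in Tick alongside the elapsed and escape timers.
; Timelines drive sprint FOV and hold-or-toggle crouch capsule height, while P pauses with a sensitivity slider.
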(event Custom|Stop%20Running
  (Variables|/Script/Engine.CharacterMovementComponent|SetMaxWalkSpeed (Variables|Character|GetCharacterMovement) 6e+02)
  (bind _fov (Timeline|fov Reverse)
    (:Update
      (Variables|/Script/Engine.PlayerCameraManager|SetDefaultFOV (Game|GetPlayerCameraManager 0) _fov))))

(event Custom|Custom%20Un%20Crunch
  (Variables|Default|SetbCrunching false)
  (Variables|/Script/Engine.CharacterMovementComponent|SetMaxWalkSpeed (Variables|Character|GetCharacterMovement) 6e+02)
  (bind _hal_higth (Timeline|crunch_time Reverse)
    (:Update
      (Components|Capsule|SetCapsuleHalfHeight (Variables|Collision|GetCapsuleComponent) _hal_higth true))))

(event Custom|Custom%20Crunch
  (Variables|Default|SetbCrunching true)
  (CallFunction|StopRunning)
  (Variables|/Script/Engine.CharacterMovementComponent|SetMaxWalkSpeed (Variables|Character|GetCharacterMovement) 4e+02)
  (bind _hal_higth (Timeline|crunch_time Play)
    (:Update
      (Components|Capsule|SetCapsuleHalfHeight (Variables|Collision|GetCapsuleComponent) _hal_higth true))))

(event Custom|LigarCameraLenta
  (Default|CallAvisarMudancaTempo)
  (Variables|Default|SetbEstadoDeBarraCameraLenta? true)
  (Variables|Default|SetCompensasao (/ 1.0 (Class|GameplayStatics|GetGlobalTimeDilation)))
  (Utilities|Time|SetGlobalTimeDilation 0.2)
  (Variables|/Script/Engine.Actor|SetCustomTimeDilation (Game|GetPlayerController 0) (Variables|Default|GetCompensasao)))

(event Custom|DesligarCameraLenta
  (Utilities|Time|SetGlobalTimeDilation 1.0)
  (Variables|/Script/Engine.Actor|SetCustomTimeDilation (Game|GetPlayerController 0) 1.0)
  (Variables|Default|SetbEstadoDeBarraCameraLenta? false))

(event Input|EnhancedActionEvents|EnhancedInputActionIA_Moviment
  (params (ActionValue :type Vector%202D%20Structure) (ElapsedSeconds :type Float%20%28double-precision%29) (TriggeredSeconds :type Float%20%28double-precision%29) (InputAction :type Input%20Action%20Object%20Reference :default "/Game/Inputs/IA_Moviment.IA_Moviment"))
  (bind (_x _y) (Math|Vector2D|BreakVector2D ActionValue))
  (Pawn|Input|AddMovementInput (* (Transformation|GetActorForwardVector) _y) 1.0 false)
  (Pawn|Input|AddMovementInput (* (Transformation|GetActorRightVector) _x) 1.0 false))

(event Input|EnhancedActionEvents|EnhancedInputActionIA_Look_d
  (params (ActionValue :type Vector%202D%20Structure) (ElapsedSeconds :type Float%20%28double-precision%29) (TriggeredSeconds :type Float%20%28double-precision%29) (InputAction :type Input%20Action%20Object%20Reference :default "/Game/Inputs/IA_Look_d.IA_Look_d"))
  (bind (_x _y) (Math|Vector2D|BreakVector2D ActionValue))
  (Pawn|Input|AddControllerPitchInput (* (* _y -1.0) (Variables|Default|GetMouseSensitivity)))
  (Pawn|Input|AddControllerYawInput (* _x (Variables|Default|GetMouseSensitivity))))

(event Input|EnhancedActionEvents|EnhancedInputActionIA_Running
  (params (ActionValue :type Boolean) (ElapsedSeconds :type Float%20%28double-precision%29) (TriggeredSeconds :type Float%20%28double-precision%29) (InputAction :type Input%20Action%20Object%20Reference :default "/Game/Inputs/IA_Running.IA_Running"))
  (:Triggered
    (if (not (AI|Components|NavMovement|IsFalling (Variables|Character|GetCharacterMovement)))
      (if (not (Variables|Default|GetbCrunching))
        (Variables|/Script/Engine.CharacterMovementComponent|SetMaxWalkSpeed (Variables|Character|GetCharacterMovement) 1.5e+03)
        (bind _fov (Timeline|fov PlayFromStart)
          (:Update
            (Variables|/Script/Engine.PlayerCameraManager|SetDefaultFOV (Game|GetPlayerCameraManager 0) _fov))))))
  (:Completed
    (CallFunction|StopRunning)))

(event Input|EnhancedActionEvents|EnhancedInputActionIA_MyJumpig
  (params (ActionValue :type Boolean) (ElapsedSeconds :type Float%20%28double-precision%29) (TriggeredSeconds :type Float%20%28double-precision%29) (InputAction :type Input%20Action%20Object%20Reference :default "/Game/Inputs/IA_MyJumpig.IA_MyJumpig"))
  (:Triggered
    (Character|Jump)
    (CallFunction|StopRunning))
  (:Completed
    (Character|StopJumping)))

(event Input|EnhancedActionEvents|EnhancedInputActionIA_Crunch
  (params (ActionValue :type Boolean) (ElapsedSeconds :type Float%20%28double-precision%29) (TriggeredSeconds :type Float%20%28double-precision%29) (InputAction :type Input%20Action%20Object%20Reference :default "/Game/Inputs/IA_Crunch.IA_Crunch"))
  (:Triggered
    (Utilities|FlowControl|DoOnce false :!label _label
      (:Completed
        (if (Variables|Default|GetbHoldingCrounch)
          (CallFunction|CustomCrunch)
          (else
            (Utilities|FlowControl|FlipFlop
              (:A
                (CallFunction|CustomCrunch))
              (:B
                (CallFunction|CustomUnCrunch))))))))
  (:Completed
    (Utilities|FlowControl|Sequence
      (:then_0
        (if (Variables|Default|GetbHoldingCrounch)
          (CallFunction|CustomUnCrunch)))
      (:then_1
        (goto _label Reset)))))

(event Input|EnhancedActionEvents|EnhancedInputActionIA_Pause
  (params (ActionValue :type Boolean) (ElapsedSeconds :type Float%20%28double-precision%29) (TriggeredSeconds :type Float%20%28double-precision%29) (InputAction :type Input%20Action%20Object%20Reference :default "/Game/Inputs/IA_Pause.IA_Pause")))

(event EventBeginPlay
  (Input|AddMappingContext (PlayerController|LocalPlayerSubsystems|GetEnhancedInputLocalPlayerSubsystem (Game|GetPlayerController 0)) "/Game/Inputs/IMC_Defalt.IMC_Defalt" 0 "(bIgnoreAllPressedKeysUntilRelease=True,bForceImmediately=False,bNotifyUserSettings=False)")
  (bind _returnvalue (Game|SpawnActorfromClass "/Game/BP_Wepon1.BP_Wepon1_C" (Math|Transform|MakeTransform "-10.000000,26.666667,15.000000" "0, 0, 0" "1.000000,1.000000,1.000000") "Undefined" "MultiplyWithRoot" 0 self))
  (bind _output_get (Variables|Default|SetcurrentWepon _returnvalue))
  (Transformation|AttachComponentToComponent _output_get (Variables|Default|GetSK_TriggerBurst1) "head" "KeepRelative" "KeepWorld" "KeepRelative" true)
  (Variables|Default|SetTyper%20Wepon (Variables|/Game/BP_Wepon1.BP_Wepon1_C|GetTyperWepon _output_get))
  (bind _returnvalue_2 (UserInterface|CreateWidget "/Game/WD_CrossHair.WD_CrossHair_C"))
  (UserInterface|Viewport|AddtoViewport _returnvalue_2 0)
  (bind _returnvalue_3 (UserInterface|CreateWidget "/Game/WD_BarCameraLenta.WD_BarCameraLenta_C"))
  (UserInterface|Viewport|AddtoViewport _returnvalue_3 0)
  (bind _returnvalue_4 (UserInterface|CreateWidget "/Game/WD_Timer.WD_Timer_C"))
  (UserInterface|Viewport|AddtoViewport _returnvalue_4 0)
  (Variables|Default|SetTempoDeFuga 6e+01))

(event Collision|EventActorBeginOverlap
  (params (OtherActor :type Actor%20Object%20Reference)))

(event EventTick
  (params (DeltaSeconds :type Float%20%28single-precision%29))
  (if (Variables|Default|GetbTimerEstaCorrendo)
    (Variables|Default|SetTempoTotalDeJogo (+ DeltaSeconds (Variables|Default|GetTempoTotalDeJogo))))
  (if (Variables|Default|GetbContagemRegressivaEstaCorrendo) :!label _label
    (bind _output_get (Variables|Default|SetTempoDeFuga (Math|Float|Clamp(Float) (- (Variables|Default|GetTempoDeFuga) DeltaSeconds) 0.0 6e+01)))
    (Variables|Default|SetTempoTotalDeJogo (+ DeltaSeconds (Variables|Default|GetTempoTotalDeJogo)))
    (if (<= _output_get 0.0)
      (goto _label)
      (else
        _)))
  (Variables|Default|SetPePos (Transformation|GetWorldLocation (Variables|Default|GetPé)))
  ;[0.15 0.15 0.15 0.5] ControladorDeEstaminaDaCameraLenta
  (Transformation|SetRelativeRotation (Variables|Default|Getpivot) (Math|Rotator|MakeRotator 0.0 (.Pitch (Math|Rotator|BreakRotator (Pawn|GetControlRotation :!class /Script/Engine.Pawn))) 0.0) false false)
  (if (Variables|Default|GetbEstadoDeBarraCameraLenta?)
    (if (>= (- (Variables|Default|GetStaminaCameraLenta) (* (Variables|Default|GetTaxaDeDreno) DeltaSeconds)) 0.0)
      (Variables|Default|SetStaminaCameraLenta (Math|Float|Clamp(Float) (- (Variables|Default|GetStaminaCameraLenta) (* (Variables|Default|GetTaxaDeDreno) DeltaSeconds)) 0.0 (Variables|Default|GetMaxStaminaCameraLenta)))
      (else
        (CallFunction|DesligarCameraLenta)))
    (else
      (Variables|Default|SetStaminaCameraLenta (Math|Float|Clamp(Float) (+ (Variables|Default|GetStaminaCameraLenta) (* (Variables|Default|GetTaxaDeRecargaStamina) DeltaSeconds)) 0.0 (Variables|Default|GetMaxStaminaCameraLenta))))))

(event Input|MouseEvents|LeftMouseButton
  (params (Key :type Key%20Structure :default "None"))
  (bind _camera (Variables|Default|GetCamera))
  (bind _returnvalue (Transformation|GetWorldRotation _camera))
  (:Pressed
    (bind _output_get (Variables|Default|SetbFiring? true))
    (if _output_get
      (Game|Feedback|ClientStartCameraShake (Game|GetPlayerController 0) "/Game/BP_CameraShakeTiro.BP_CameraShakeTiro_C" 1.0 "CameraLocal" "0, 0, 0")
      (Game|SpawnActorfromClass "/Game/BP_Bullet.BP_Bullet_C" (Math|Transform|MakeTransform (Transformation|GetWorldLocation (Variables|/Game/BP_Wepon1.BP_Wepon1_C|GetScene1 (Variables|Default|GetcurrentWepon))) (Math|Rotator|MakeRotator (.roll _returnvalue) (.pitch _returnvalue) (+ (.yaw _returnvalue) -0.2)) "1.000000,1.000000,1.000000") "Undefined" "MultiplyWithRoot" 0 0)))
  (:Released
    (Variables|Default|SetbFiring? false)))

(event Input|MouseEvents|RightMouseButton
  (params (Key :type Key%20Structure :default "None"))
  (:Pressed
    (if (> (Variables|Default|GetStaminaCameraLenta) 0.0)
      (CallFunction|LigarCameraLenta)))
  (:Released
    (CallFunction|DesligarCameraLenta)))

(event Input|KeyboardEvents|P
  (params (Key :type Key%20Structure :default "None"))
  (:Pressed
    (if (Variables|Default|GetPause)
      (Game|SetGamePaused false)
      (Variables|/Script/Engine.PlayerController|SetbShowMouseCursor (Game|GetPlayerController 0) false)
      (Widget|RemovefromParent (Variables|Default|GetSensebility))
      (Input|SetInputModeGameOnly (Game|GetPlayerController 0) false)
      (Variables|Default|SetPause false)
      (else
        (Game|SetGamePaused true)
        (Variables|/Script/Engine.PlayerController|SetbShowMouseCursor (Game|GetPlayerController 0) true)
        (bind _returnvalue (UserInterface|CreateWidget "/Game/WD_SliderSensibility.WD_SliderSensibility_C"))
        (bind _output_get (Variables|Default|SetSensebility _returnvalue))
        (UserInterface|Viewport|AddtoViewport _output_get 0)
        (Input|SetInputModeGameandUI (Game|GetPlayerController 0) (Variables|Default|GetSensebility) "DoNotLock" true false)
        (Variables|Default|SetPause true)))))

(fn ConstructionScript)