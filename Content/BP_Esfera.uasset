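; BP_Esfera is a lethal energy sphere that grows once the player's PressPilar flag is set.
; Tick polls that flag on the cached BP_Player, reveals the Energia component and steadily increases its world scale.
; When Energia hits the player, it blocks move and look input, shows the WBP_TelaMorte death screen, then after a short delay saves the level's play time in GI_GerenciadorJogo and reloads the level.
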(event OnComponentHit(Energia)
  (params (HitComponent :type Primitive%20Component%20Object%20Reference) (OtherActor :type Actor%20Object%20Reference) (OtherComp :type Primitive%20Component%20Object%20Reference) (NormalImpulse :type Vector :default "0, 0, 0") (Hit :type Hit%20Result%20Structure%20%28by%20ref%29))
  (bind _asbp_player (Utilities|Casting|CastToBP_Player OtherActor))
  (bind _output_get (Variables|Default|SetAs%20BP%20Player _asbp_player))
  (Input|SetIgnoreMoveInput (Game|GetPlayerController 0) true)
  (Input|SetIgnoreLookInput (Game|GetPlayerController 0) true)
  (bind _returnvalue (UserInterface|CreateWidget "/Game/Widet/WBP_TelaMorte.WBP_TelaMorte_C"))
  (UserInterface|Viewport|AddtoViewport _returnvalue 0)
  (Utilities|FlowControl|Delay 2.0)
  (bind _returnvalue_2 (Game|GetCurrentLevelName true))
  (bind _asgi_gerenciador_jogo (Utilities|Casting|CastToGI_GerenciadorJogo (Game|GetGameInstance)))
  (Utilities|Map|Add (Variables|/Game/GameInstance/GI_GerenciadorJogo.GI_GerenciadorJogo_C|GetTempoDasFases _asgi_gerenciador_jogo) _returnvalue_2 (Variables|/Game/BP_Player.BP_Player_C|GetTempoTotalDeJogo _output_get))
  (Game|OpenLevel(byName) (Utilities|String|StringToName _returnvalue_2)))

(event EventBeginPlay
  (bind _asbp_player (Utilities|Casting|CastToBP_Player (Game|GetPlayerCharacter 0)))
  (Variables|Default|SetAs%20BP%20Player _asbp_player))

(event Collision|EventActorBeginOverlap
  (params (OtherActor :type Actor%20Object%20Reference)))

(event EventTick
  (params (DeltaSeconds :type Float%20%28single-precision%29))
  (if (Variables|/Game/BP_Player.BP_Player_C|GetbPressPilar (Variables|Default|GetAs%20BP%20Player))
    (Rendering|SetVisibility (Variables|Default|GetEnergia) true false)
    (bind _output_get (Variables|Default|SetEscalaAtual (+ (Variables|Default|GetEscalaAtual) (* DeltaSeconds 3.0))))
    (Transformation|SetWorldScale3D (Variables|Default|GetEnergia) (Math|Conversions|ToVector(Float) _output_get))))

(fn ConstructionScript)