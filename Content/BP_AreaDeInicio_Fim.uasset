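; BP_AreaDeInicio_Fim is a trigger area that serves as both the start and finish zone for the player's timed escape.
; When BP_Player enters the Box, it sets the player's Terminou (finished) flag if TempoDeFuga (escape time) equals exactly zero.
; When BP_Player leaves the Box, it sets TimerEstaCorrendo to mark the timer as running.
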(event OnComponentEndOverlap(Box)
  (params (OverlappedComponent :type Primitive%20Component%20Object%20Reference) (OtherActor :type Actor%20Object%20Reference) (OtherComp :type Primitive%20Component%20Object%20Reference) (OtherBodyIndex :type Integer))
  (bind _asbp_player (Utilities|Casting|CastToBP_Player OtherActor))
  (bind _output_get (Variables|Default|SetPlayer _asbp_player))
  (Variables|/Game/BP_Player.BP_Player_C|SetbTimerEstaCorrendo _output_get true))

(event OnComponentBeginOverlap(Box)
  (params (OverlappedComponent :type Primitive%20Component%20Object%20Reference) (OtherActor :type Actor%20Object%20Reference) (OtherComp :type Primitive%20Component%20Object%20Reference) (OtherBodyIndex :type Integer) (bFromSweep :type Boolean) (SweepResult :type Hit%20Result%20Structure%20%28by%20ref%29))
  (bind _asbp_player (Utilities|Casting|CastToBP_Player OtherActor))
  (Variables|Default|SetPlayer _asbp_player)
  (if (== (Variables|/Game/BP_Player.BP_Player_C|GetTempoDeFuga (Variables|Default|GetPlayer)) 0.0)
    (Variables|/Game/BP_Player.BP_Player_C|SetbTerminou (Variables|Default|GetPlayer) true)))

(event EventBeginPlay)

(event Collision|EventActorBeginOverlap
  (params (OtherActor :type Actor%20Object%20Reference)))

(event EventTick
  (params (DeltaSeconds :type Float%20%28single-precision%29)))

(fn ConstructionScript)