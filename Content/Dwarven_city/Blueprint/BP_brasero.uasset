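; Brazier interactable in the Dwarven city that, on a one-time player press, opens a scroll text widget and reveals a portal's vortex and sparks.
; Box overlap caches the player, sets their pillar-interaction flag and toggles an overlay highlight and prompt texts.
; Tick turns the prompt toward the camera and polls the player's press, then shows return text and a "RUNN!!!!!!" warning.
; Leaving the box hides the prompts but leaves both interaction flags set.
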(event OnComponentBeginOverlap(Box)
  (params (OverlappedComponent :type Primitive%20Component%20Object%20Reference) (OtherActor :type Actor%20Object%20Reference) (OtherComp :type Primitive%20Component%20Object%20Reference) (OtherBodyIndex :type Integer) (bFromSweep :type Boolean) (SweepResult :type Hit%20Result%20Structure%20%28by%20ref%29))
  (bind _asbp_player (Utilities|Casting|CastToBP_Player OtherActor))
  (bind _output_get (Variables|Default|SetOverley "/Game/Materials/MAT_OverlayMaterial.MAT_OverlayMaterial"))
  (Rendering|Material|SetOverlayMaterial (Variables|Default|GetCube) _output_get :!class /Script/Engine.MeshComponent)
  (Variables|Default|SetPlayer _asbp_player)
  (Rendering|SetVisibility (Variables|Default|GetTextRender) true false)
  (Rendering|SetVisibility (Variables|Default|GetText) true false)
  (Variables|Default|SetbPlayerAndando true)
  (Variables|/Game/BP_Player.BP_Player_C|SetinteraçãoDoPilar (Variables|Default|GetPlayer) true))

(event OnComponentEndOverlap(Box)
  (params (OverlappedComponent :type Primitive%20Component%20Object%20Reference) (OtherActor :type Actor%20Object%20Reference) (OtherComp :type Primitive%20Component%20Object%20Reference) (OtherBodyIndex :type Integer))
  (bind _asbp_player (Utilities|Casting|CastToBP_Player OtherActor))
  (Rendering|Material|SetOverlayMaterial (Variables|Default|GetCube) 0 :!class /Script/Engine.MeshComponent)
  (Variables|Default|SetPlayer _asbp_player)
  (Rendering|SetVisibility (Variables|Default|GetTextRender) false false)
  (Rendering|SetVisibility (Variables|Default|GetText) false false))

(event EventBeginPlay)

(event Collision|EventActorBeginOverlap
  (params (OtherActor :type Actor%20Object%20Reference)))

(event EventTick
  (params (DeltaSeconds :type Float%20%28single-precision%29))
  (if (not (Variables|Default|GetbJáEntou))
    (Variables|Default|GetPlayer
      (:then
        (if (Variables|Default|GetbPlayerAndando)
          (Transformation|SetWorldRotation (Variables|Default|GetTextRender) (Math|Rotator|FindLookatRotation (Transformation|GetWorldLocation (Variables|Default|GetTextRender)) (Camera|GetCameraLocation (Game|GetPlayerCameraManager 0))) false false)
          (if (Variables|/Game/BP_Player.BP_Player_C|GetbPressPilar (Variables|Default|GetPlayer))
            (bind _returnvalue (UserInterface|CreateWidget "/Game/Widet/WBP_TextoScroll.WBP_TextoScroll_C"))
            (UserInterface|Viewport|AddtoViewport _returnvalue 0)
            (Rendering|SetVisibility (Variables|Default|GetTextReturn) true false)
            (Rendering|SetVisibility (Variables|/Game/AdvancedPortalsSystemVFX/Blueprints/BP_Portal_6.BP_Portal_6_C|GetVortex (Variables|Default|GetPortalInteração)) true false)
            (Rendering|SetVisibility (Variables|/Game/AdvancedPortalsSystemVFX/Blueprints/BP_Portal_6.BP_Portal_6_C|GetSparks_1 (Variables|Default|GetPortalInteração)) true false)
            (Rendering|Components|TextRender|SetText (Variables|Default|GetTextRender) (Utilities|Text|ToText(String) "RUNN!!!!!!"))
            (Variables|Default|SetbJáEntou true))))
      (:else))))

(fn ConstructionScript)