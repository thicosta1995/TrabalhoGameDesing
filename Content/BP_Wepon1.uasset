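; Weapon actor Blueprint that fires projectiles through a shoot event.
; Shoot raises global time dilation, speeding up the whole game without resetting it here, then spawns BP_Bullet at the Scene1 component's location and rotation.
; A separate CreateShoot event line-traces forward from the Arrow over a given Range for pawns, but ignores the hits.
; Leftover trace and debug-print nodes are unconnected.
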(event Custom|CreateShoot
  (params (Range :type Float%20%28double-precision%29))
  (bind _arrow (Variables|Default|GetArrow))
  (bind _returnvalue (Transformation|GetWorldLocation _arrow))
  (Class|KismetSystemLibrary|LineTraceMultiforObjects _returnvalue (+ _returnvalue (* (Math|Vector|GetForwardVector (Transformation|GetWorldRotation _arrow)) Range)) (Utilities|Array|MakeArray "ObjectTypeQuery3") false 0 "None" true))

(event Custom|shoot
  (bind _scene1 (Variables|Default|GetScene1))
  (Utilities|Time|SetGlobalTimeDilation 5.0)
  (Game|SpawnActorfromClass "/Game/BP_Bullet.BP_Bullet_C" (Math|Transform|MakeTransform (Transformation|GetWorldLocation _scene1) (Transformation|GetWorldRotation _scene1) "1.000000,1.000000,1.000000") "Undefined" "MultiplyWithRoot" 0 0))

(event EventBeginPlay)

(event Collision|EventActorBeginOverlap
  (params (OtherActor :type Actor%20Object%20Reference)))

(event EventTick
  (params (DeltaSeconds :type Float%20%28single-precision%29)))

(fn ConstructionScript)